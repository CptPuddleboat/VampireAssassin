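; MovingCar_BP is an environment actor that loops a car along a path between two points in the level.
; On BeginPlay it snaps the Car component to PointA, waits a random few seconds, then uses MoveComponentTo to glide it to PointA1's relative location and rotation.
; After a short pause the sequence re-enters through a Gate and repeats, so the car reappears at the start at irregular intervals.
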(event `self.ReceiveBeginPlay`
  (bind _car (`self.Car`))
  (`/Engine/EditorBlueprintResources/StandardMacros.Gate` false :!label _label
    (:`Exit`
      (`SceneComponent.K2_SetWorldLocation` _car (`SceneComponent.K2_GetComponentLocation` (`self.PointA`)) false false)
      (`KismetSystemLibrary.Delay` (`KismetMathLibrary.RandomFloatInRange` 1.0 10.0))
      (`KismetSystemLibrary.MoveComponentTo` _car (.location (`SceneComponent.GetRelativeTransform` (`self.PointA1`))) (.rotation (`SceneComponent.GetRelativeTransform` (`self.PointA1`))) false false 20.0)
      (`KismetSystemLibrary.Delay` 1.0)
      (goto _label))))

(fn `UserConstructionScript`)