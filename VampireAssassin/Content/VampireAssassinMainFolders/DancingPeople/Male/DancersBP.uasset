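; Dancing crowd NPC whose blood can be drained, destroyed when it runs out.
; BeginPlay randomly picks a male or female mesh, randomizes its materials, then loops one of that gender's dances after a random delay to stagger the crowd.
; SetDrain toggles draining, which lowers Blood on Tick and updates a text display; at zero, Die clears Damian's Draining flag.
; The function to turn the text toward the player is disconnected.
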(event `self.ReceiveBeginPlay`
  (bind _mesh (`self.Mesh`))
  ;[1 1 1] Aniamtion to play
  (switch `int` (`KismetMathLibrary.RandomIntegerInRange` 0 1)
    (:`0`
      (`SkinnedMeshComponent.SetSkinnedAssetAndUpdate` _mesh "/Game/VampireAssassinMainFolders/DancingPeople/Male/Male_Mesh.Male_Mesh" true)
      (`self.Male Items`))
    (:`1`
      (`SkinnedMeshComponent.SetSkinnedAssetAndUpdate` _mesh "/Game/VampireAssassinMainFolders/DancingPeople/Female/Female_Mesh.Female_Mesh" true)
      (`self.Female Items`))))

(event `Female Items`
  (bind _returnvalue (`KismetMathLibrary.RandomFloatInRange` 0.1 2.0))
  (bind _mesh (`self.Mesh`))
  ;[1 1 1] Aniamtion to play
  ;;[1 1 1] Female BP
  ;;;[1 1 1] Color of Character
  (`self.Color Picking for females`)
  (switch `int` (`KismetMathLibrary.RandomIntegerInRange` 0 3)
    (:`0`
      (`KismetSystemLibrary.Delay` _returnvalue)
      (`SkeletalMeshComponent.PlayAnimation` _mesh "/Game/VampireAssassinMainFolders/DancingPeople/Female/Animations/Hip_Hop_Dancing.Hip_Hop_Dancing" true))
    (:`1`
      (`KismetSystemLibrary.Delay` _returnvalue)
      (`SkeletalMeshComponent.PlayAnimation` _mesh "/Game/VampireAssassinMainFolders/DancingPeople/Female/Animations/Hip_Hop_Dancing_v2_Anim.Hip_Hop_Dancing_v2_Anim" true))
    (:`2`
      (`KismetSystemLibrary.Delay` _returnvalue)
      (`SkeletalMeshComponent.PlayAnimation` _mesh "/Game/VampireAssassinMainFolders/DancingPeople/Female/Animations/Hip_Hop_Dancing_v3.Hip_Hop_Dancing_v3" true))
    (:`3`
      (`KismetSystemLibrary.Delay` _returnvalue)
      (`SkeletalMeshComponent.PlayAnimation` _mesh "/Game/VampireAssassinMainFolders/DancingPeople/Female/Animations/Rumba_Dancing.Rumba_Dancing" true))))

(event `Male Items`
  (bind _returnvalue (`KismetMathLibrary.RandomFloatInRange` 0.1 2.0))
  (bind _mesh (`self.Mesh`))
  ;[1 1 1] Aniamtion to play
  ;;[1 1 1] Male BP
  ;;;[1 1 1] Color of Character
  (`self.Color Picking for males`)
  (switch `int` (`KismetMathLibrary.RandomIntegerInRange` 0 3)
    (:`0`
      (`KismetSystemLibrary.Delay` _returnvalue)
      (`SkeletalMeshComponent.PlayAnimation` _mesh "/Game/VampireAssassinMainFolders/DancingPeople/Male/Animations/Hip_Hop_Dancing.Hip_Hop_Dancing" true))
    (:`1`
      (`KismetSystemLibrary.Delay` _returnvalue)
      (`SkeletalMeshComponent.PlayAnimation` _mesh "/Game/VampireAssassinMainFolders/DancingPeople/Male/Animations/House_Dancing.House_Dancing" true))
    (:`2`
      (`KismetSystemLibrary.Delay` _returnvalue)
      (`SkeletalMeshComponent.PlayAnimation` _mesh "/Game/VampireAssassinMainFolders/DancingPeople/Male/Animations/Salsa_Dancing_Anim.Salsa_Dancing_Anim" true))
    (:`3`
      (`KismetSystemLibrary.Delay` _returnvalue)
      (`SkeletalMeshComponent.PlayAnimation` _mesh "/Game/VampireAssassinMainFolders/DancingPeople/Male/Animations/Silly_Dancing.Silly_Dancing" true))))

(event `self.ReceiveTick`
  (params (DeltaSeconds :type "Float (single-precision)"))
  ;[1 1 1] Draining
  (`self.MakeTextFacePlayer`)
  (if (`self.IsBeingDrained`)
    (bind _output_get (set `self.Blood` (- (`self.Blood`) (* 50.0 DeltaSeconds))))
    (`TextRenderComponent.K2_SetText` (`self.TextRender`) (`KismetTextLibrary.Conv_DoubleToText` _output_get "HalfToEven"))
    (if (<= _output_get 0.0)
      (`self.Die`))))

(event `Die`
  ;[1 1 1] Draining
  (set `self.Dead` true)
  (set `self.IsBeingDrained` false)
  (`TextRenderComponent.K2_SetText` (`self.TextRender`) (`KismetTextLibrary.Conv_StringToText` "DEAD"))
  (bind _asdamian (cast `/Game/VampireAssassinMainFolders/Character/PlayerCharacter/Damian` (`GameplayStatics.GetPlayerPawn` 0)))
  (set `/Game/VampireAssassinMainFolders/Character/PlayerCharacter/Damian.Draining` false _asdamian)
  (`self.K2_DestroyActor`))

(event `SetDrain`
  (params (BeingDrained :type Boolean))
  ;[1 1 1] Draining
  (set `self.IsBeingDrained` BeingDrained))

(fn `Color Picking for females`
  (bind _returnvalue (`KismetMathLibrary.RandomIntegerInRange` 0 2))
  (`PrimitiveComponent.SetMaterial` (`self.Mesh`) 0 (`|GetArrayItem` (`self.SkinColors`) (`KismetMathLibrary.RandomIntegerInRange` 0 2)))
  (`PrimitiveComponent.SetMaterial` (`self.Mesh`) 1 (`|GetArrayItem` (`self.DressColors`) _returnvalue))
  (`PrimitiveComponent.SetMaterial` (`self.Mesh`) 2 "/Game/VampireAssassinMainFolders/DancingPeople/MATS/Eyes.Eyes")
  (`PrimitiveComponent.SetMaterial` (`self.Mesh`) 3 (`|GetArrayItem` (`self.HairColors`) (`KismetMathLibrary.RandomIntegerInRange` 0 3)))
  (`PrimitiveComponent.SetMaterial` (`self.Mesh`) 4 (`|GetArrayItem` (`self.DressColors`) _returnvalue)))

(fn `Color Picking for males`
  (`PrimitiveComponent.SetMaterial` (`self.Mesh`) 0 (`|GetArrayItem` (`self.SkinColors`) (`KismetMathLibrary.RandomIntegerInRange` 0 2)))
  (`PrimitiveComponent.SetMaterial` (`self.Mesh`) 1 "/Game/VampireAssassinMainFolders/DancingPeople/MATS/Eyes.Eyes")
  (`PrimitiveComponent.SetMaterial` (`self.Mesh`) 2 (`|GetArrayItem` (`self.JacketColors`) (`KismetMathLibrary.RandomIntegerInRange` 0 3)))
  (`PrimitiveComponent.SetMaterial` (`self.Mesh`) 3 (`|GetArrayItem` (`self.T-ShirtColors`) (`KismetMathLibrary.RandomIntegerInRange` 0 5)))
  (`PrimitiveComponent.SetMaterial` (`self.Mesh`) 4 (`|GetArrayItem` (`self.SeemColors`) (`KismetMathLibrary.RandomIntegerInRange` 0 1)))
  (`PrimitiveComponent.SetMaterial` (`self.Mesh`) 4 (`|GetArrayItem` (`self.PantsColors`) (`KismetMathLibrary.RandomIntegerInRange` 0 1)))
  (`PrimitiveComponent.SetMaterial` (`self.Mesh`) 4 (`|GetArrayItem` (`self.ShoesColors`) (`KismetMathLibrary.RandomIntegerInRange` 0 1))))

(fn `MakeTextFacePlayer`)

(fn `UserConstructionScript`
  (`TextRenderComponent.K2_SetText` (`self.TextRender`) (`KismetTextLibrary.Conv_DoubleToText` (`self.Blood`) "HalfToEven")))