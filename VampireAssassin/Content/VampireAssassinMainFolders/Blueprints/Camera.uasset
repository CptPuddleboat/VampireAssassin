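; Follow camera actor that tracks a target, by default the Damian player, rotates from input scaled by sensitivity, and supports temporary retargeting.
; Each tick it snaps to the target and traces from the cine camera to its root to test player visibility.
; When blocked, it drives PC_Data material parameters and positions two sphere mask child actors, likely for see-through occlusion.
; It also yaws the player's Detection component toward the camera.
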(event `self.ReceiveTick`
  (params (DeltaSeconds :type "Float (single-precision)"))
  (`|ExecutionSequence`
    (:`then_0`
      (`self.K2_SetActorLocation` (`self.K2_GetActorLocation` (`self.target`)))
      (bind _outhit (`KismetSystemLibrary.LineTraceSingle` (`SceneComponent.K2_GetComponentLocation` (`self.CineCamera`)) (`SceneComponent.K2_GetComponentLocation` (`self.DefaultSceneRoot`)) "TraceTypeQuery1"))
      (if (== (`.HitActor` (`GameplayStatics.BreakHitResult` _outhit)) (`self.player`))
        (set `self.CanSeePlayer` true)
        (`KismetMaterialLibrary.SetScalarParameterValue` "/Game/Mask-DontWorry/PC_Data.PC_Data" "BooleanCheck")
        (`KismetMaterialLibrary.SetScalarParameterValue` "/Game/Mask-DontWorry/PC_Data.PC_Data" "Radius")
        (`/Game/Mask-DontWorry/BP_Sphere.GoAway` (`self.MaskBoxRef`))
        (`/Game/Mask-DontWorry/BP_Sphere2.GoAway` (`self.MaskBox2Ref`))
        (else
          (set `self.CanSeePlayer` false)
          (`KismetMaterialLibrary.SetScalarParameterValue` "/Game/Mask-DontWorry/PC_Data.PC_Data" "BooleanCheck" 1.0)
          (`/Game/Mask-DontWorry/BP_Sphere.MaskLocation` (`self.MaskBoxRef`))
          (`/Game/Mask-DontWorry/BP_Sphere2.MaskLocation` (`self.MaskBox2Ref`)))))
    (:`then_1`
      (`self.Set Rotation`))))

(event `self.ReceiveBeginPlay`
  (bind _returnvalue (`GameplayStatics.GetPlayerController` 0))
  (`|ExecutionSequence`
    (:`then_0`
      (bind _asvampire_assassin_game_instance (cast `/Game/UE4Character/Game/VampireAssassinGameInstance` (`GameplayStatics.GetGameInstance`)))
      (set `self.GameInstanceRef` _asvampire_assassin_game_instance))
    (:`then_1`
      (`self.EventBinds`)
      (bind _asdamian (cast `/Game/VampireAssassinMainFolders/Character/PlayerCharacter/Damian` (`Controller.K2_GetPawn` _returnvalue)))
      (bind _output_get (set `self.player` _asdamian))
      (if (`self.beginTargetPlayer`)
        (set `self.target` _output_get)
        (`PlayerController.SetViewTargetWithBlend` _returnvalue self 0.0 "VTBlend_Linear" 0.0 false)
        (bind _asbp_sphere (cast `/Game/Mask-DontWorry/BP_Sphere` (`ChildActorComponent.ChildActor` (`self.MaskBox1`))))
        (set `self.MaskBoxRef` _asbp_sphere)
        (bind _asbp_sphere_2 (cast `/Game/Mask-DontWorry/BP_Sphere2` (`ChildActorComponent.ChildActor` (`self.MaskBox2`))))
        (set `self.MaskBox2Ref` _asbp_sphere_2)))))

(event `SetTarget`
  (params (targetActor :type "Actor Object Reference"))
  (set `self.target` targetActor))

(event `SetTemporaryTarget`
  (params (targetActor :type "Actor Object Reference") (Time :type "Float (double-precision)"))
  (set `self.storeTarget` (`self.target`))
  (set `self.target` targetActor)
  (`KismetSystemLibrary.Delay` Time)
  (set `self.target` (`self.storeTarget`)))

(event `EventBinds`
  (add `self.E_CameraRotate` (delegate `CameraRotate`)))

(event `Set Rotation`
  (bind _detection (`/Game/VampireAssassinMainFolders/Character/PlayerCharacter/Damian.Detection` (`self.player`)))
  (bind (_returnvalue_roll _returnvalue_pitch _returnvalue_yaw) (`KismetMathLibrary.BreakRotator` (`KismetMathLibrary.FindLookAtRotation` (`SceneComponent.K2_GetComponentLocation` _detection) (`SceneComponent.K2_GetComponentLocation` (`self.CineCamera`)))))
  (`SceneComponent.K2_SetWorldRotation` _detection (`KismetMathLibrary.MakeRotator` 0.0 0.0 (+ _returnvalue_yaw (stale `CameraRotate` Axis))) false false :!label _label))

(event `CameraRotate` :!signature `self.E_CameraRotate`
  (params (Axis :type "Float (double-precision)"))
  (bind (_returnvalue_roll _returnvalue_pitch _returnvalue_yaw) (`KismetMathLibrary.BreakRotator` (`self.K2_GetActorRotation`)))
  (`self.K2_SetActorRotation` (`KismetMathLibrary.MakeRotator` _returnvalue_roll _returnvalue_pitch (+ _returnvalue_yaw (* Axis (+ (`/Game/UE4Character/Game/VampireAssassinGameInstance.CameraSensitivity` (`self.GameInstanceRef`)) (`self.Base Turn Speed`))))) true)
  (goto _label))

(fn `UserConstructionScript`)