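; Physics-driven double door that opens only for staff, or for anyone once the target is dead or in a tutorial level.
; A box trigger enables physics simulation on both leaves on a permitted overlap, using an interface value to tell Staff from Player, and disables it on exit.
; A blocked player reveals a text render, which end overlap also sets visible.
; A tutorial event reveals arrow decals.
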(event `Tut show Arrows`
  (for _array_element (`self.Decals`)
    (`SceneComponent.SetVisibility` (`DecalActor.Decal` _array_element) true false)))

(event `self.Box.OnComponentBeginOverlap`
  (params (OverlappedComponent :type "PrimitiveComponent Object Reference") (OtherActor :type "Actor Object Reference") (OtherComp :type "PrimitiveComponent Object Reference") (OtherBodyIndex :type Integer) (bFromSweep :type Boolean) (SweepResult :type "HitResult Structure (by ref)"))
  (if (`self.Tut Level>`)
    (`PrimitiveComponent.SetSimulatePhysics` (`self.LD`) true :!label _label)
    (`PrimitiveComponent.SetSimulatePhysics` (`self.RD`) true)
    (elif (`self.Target dead?`)
      (goto _label)
      (else
        (bind _value (message `/Game/VampireAssassinMainFolders/Blueprints/LockedDoors/GetValue.Get Value` OtherActor))
        (switch `/Game/VampireAssassinMainFolders/Blueprints/LockedDoors/CharacterValues` _value
          (:`NewEnumerator0`
            (goto _label))
          (:`NewEnumerator1`
            (`SceneComponent.SetVisibility` (`self.TextRender`) true false)))))))

(event `self.Box.OnComponentEndOverlap`
  (params (OverlappedComponent :type "PrimitiveComponent Object Reference") (OtherActor :type "Actor Object Reference") (OtherComp :type "PrimitiveComponent Object Reference") (OtherBodyIndex :type Integer))
  (`PrimitiveComponent.SetSimulatePhysics` (`self.LD`) false)
  (`PrimitiveComponent.SetSimulatePhysics` (`self.RD`) false)
  (`SceneComponent.SetVisibility` (`self.TextRender`) true false))

(fn `Get Value`
  (returns (Value :type "/Game/VampireAssassinMainFolders/Blueprints/LockedDoors/CharacterValues Enum"))
  (return "NewEnumerator0"))

(fn `UserConstructionScript`)