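; Drainable target that loses blood while the player character, presumably Damian, feeds on it, showing the remaining amount on a text render.
; SetDrain toggles draining, and Tick then lowers Blood at a fixed frame-rate-independent rate and refreshes the text, which the construction script initializes.
; At zero, Die flags the target dead, displays DEAD and clears the Draining flag on the player pawn cast to Damian.
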(event `self.ReceiveTick`
  (params (DeltaSeconds :type "Float (single-precision)"))
  (if (`self.IsBeingDrained`)
    (bind _output_get (set `self.Blood` (- (`self.Blood`) (* 50.0 DeltaSeconds))))
    (`TextRenderComponent.K2_SetText` (`self.TextRender`) (`KismetTextLibrary.Conv_DoubleToText` _output_get "HalfToEven"))
    (if (<= _output_get 0.0)
      (`self.Die`))))

(event `Die`
  (set `self.Dead` true)
  (set `self.IsBeingDrained` false)
  (`TextRenderComponent.K2_SetText` (`self.TextRender`) (`KismetTextLibrary.Conv_StringToText` "DEAD"))
  (bind _asdamian (cast `/Game/VampireAssassinMainFolders/Blueprints/Damian` (`GameplayStatics.GetPlayerPawn` 0)))
  (set `/Game/VampireAssassinMainFolders/Blueprints/Damian.Draining` false _asdamian))

(event `SetDrain`
  (params (BeingDrained :type Boolean))
  (set `self.IsBeingDrained` BeingDrained))

(fn `UserConstructionScript`
  (`TextRenderComponent.K2_SetText` (`self.TextRender`) (`KismetTextLibrary.Conv_DoubleToText` (`self.Blood`) "HalfToEven")))