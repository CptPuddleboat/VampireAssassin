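; VampireHunt is a game-level manager that sets up room lists, the match clock and the HUD at BeginPlay.
; It gathers every Zone actor and sorts it by its Restrictions value into NPC, staff or target room lists.
; A looping one-second timer drives a clock that counts seconds as separate digits and rolls them over into minutes.
; It also creates the UIManagerMaster widget, stores it as HUDRef and adds it to the viewport.
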(event `self.ReceiveBeginPlay`
  ;[1 1 1] Get all the Zones in the world
  (`|ExecutionSequence`
    (:`then_0`
      (bind _outactors (`GameplayStatics.GetAllActorsOfClass` "/Game/AI/WorldZones/Zone.Zone_C"))
      (bind _output_get (set `self.ListOfRooms` _outactors))
      (for _array_element _output_get
        (bind _restrictions (`/Game/AI/WorldZones/Zone.Restrictions` _array_element))
        ;[1 1 1] Creating Seperate lists depending on the rooms Restriction level
        (if (`KismetStringLibrary.EqualEqual_StrStr` _restrictions "All")
          (`KismetArrayLibrary.Array_Add` (`self.NPCRooms`) _array_element)
          (elif (`KismetStringLibrary.EqualEqual_StrStr` _restrictions "Staff")
            (`KismetArrayLibrary.Array_Add` (`self.StaffRooms`) _array_element)
            (elif (`KismetStringLibrary.EqualEqual_StrStr` _restrictions "Target")
              (`KismetArrayLibrary.Array_Add` (`self.TargetRooms`) _array_element))))))
    (:`then_1`
      ;[1 1 1] TimerTicks
      (bind _returnvalue (`KismetSystemLibrary.K2_SetTimerDelegate` (`|CreateDelegate` :!event `StartTimer`) 1.0 true))
      (set `self.StartTimerEventRef` _returnvalue))
    (:`then_2`
      (bind _returnvalue_2 (`|CreateWidget` "/Game/UI_Widgets/AidansUI/UIManagerMaster.UIManagerMaster_C" (`GameplayStatics.GetPlayerController` 0)))
      (bind _output_get_2 (set `self.HUDRef` _returnvalue_2))
      (`UserWidget.AddToViewport` _returnvalue_2 0)
      (`UserWidget.AddToViewport` _output_get_2 0))))

(event `StartTimer`
  ;[1 1 1] Timer
  (`self.StartTimerFunction`))

(fn `StartTimerFunction`
  ;[1 1 1] Seconds
  (set `self.Seconds` (+ (`self.Seconds`) 1))
  (if (not (<= (`self.Seconds`) 9))
    (set `self.Seconds2` (+ (`self.Seconds2`) 1))
    (set `self.Seconds` 0)
    (if (and (== (`self.Seconds2`) 6) (== (`self.Seconds`) 0))
      ;[1 1 1] Reset Seconds
      (set `self.Seconds` 0)
      (set `self.Seconds2` 0)
      ;[1 1 1] Minutes
      (set `self.Minutes` (+ (`self.Minutes`) 1)))))

(fn `UserConstructionScript`)