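; Child staff AI Blueprint that dresses a staff character to suit the level theme and tracks contact with bouncers.
; On BeginPlay it switches on LevelTheme to set the mesh and anim class for bartender, croupier, yacht crew or lifeguard roles, randomly picking between two crew variants.
; BouncerDetect overlap events filter for BouncerAI and toggle the OverlapWithBouncer blackboard key for the AI to read.
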(event `self.ReceiveBeginPlay`
  (bind _mesh (`self.Mesh`))
  (bind _mesh_2 (`self.Mesh`))
  (bind _mesh_3 (`self.Mesh`))
  (bind _mesh_4 (`self.Mesh`))
  (bind _mesh_5 (`self.Mesh`))
  (bind _mesh_6 (`self.Mesh`))
  (`parent.ReceiveBeginPlay`)
  (switch `/Game/VampireAssassinMainFolders/NPCsSkeletans/LevelThemes` (`self.LevelTheme`)
    (:`NewEnumerator0`
      (`SkinnedMeshComponent.SetSkinnedAssetAndUpdate` _mesh "/Game/VampireAssassinMainFolders/NPCsSkeletans/NightClub/Bartender/Bartender_SM.Bartender_SM" true)
      (`SkeletalMeshComponent.SetAnimInstanceClass` _mesh "/Game/VampireAssassinMainFolders/NPCsSkeletans/NightClub/Bartender/Animations/BartenderAnimBP.BartenderAnimBP_C"))
    (:`NewEnumerator1`
      (`SkinnedMeshComponent.SetSkinnedAssetAndUpdate` _mesh_3 "/Game/VampireAssassinMainFolders/NPCsSkeletans/Yatch/Bartender/Bartender_Yatch.Bartender_Yatch" true)
      (`SkeletalMeshComponent.SetAnimInstanceClass` _mesh_3 "/Game/VampireAssassinMainFolders/NPCsSkeletans/Yatch/Bartender/Animations/BartenderYatchAnimBP.BartenderYatchAnimBP_C"))
    (:`NewEnumerator2`
      (`SkinnedMeshComponent.SetSkinnedAssetAndUpdate` _mesh_6 "/Game/VampireAssassinMainFolders/NPCsSkeletans/Yatch/Cropier/croupier_idle.croupier_idle" true)
      (`SkeletalMeshComponent.SetAnimInstanceClass` _mesh_6 "/Game/VampireAssassinMainFolders/NPCsSkeletans/Yatch/Cropier/Animations/CroupierAnimBP.CroupierAnimBP_C"))
    (:`NewEnumerator3`
      (switch `int` (`KismetMathLibrary.RandomIntegerInRange` 0 1)
        (:`0`
          (`SkinnedMeshComponent.SetSkinnedAssetAndUpdate` _mesh_5 "/Game/VampireAssassinMainFolders/NPCsSkeletans/Yatch/CrewMember1/crew1_yacht_idle.crew1_yacht_idle" true)
          (`SkeletalMeshComponent.SetAnimInstanceClass` _mesh_5 "/Game/VampireAssassinMainFolders/NPCsSkeletans/Yatch/CrewMember1/Anim/Crewmem1AnimBP.Crewmem1AnimBP_C"))
        (:`1`
          (`SkinnedMeshComponent.SetSkinnedAssetAndUpdate` _mesh_2 "/Game/VampireAssassinMainFolders/NPCsSkeletans/Yatch/crewmember2/crew2_yacht_idle.crew2_yacht_idle" true)
          (`SkeletalMeshComponent.SetAnimInstanceClass` _mesh_2 "/Game/VampireAssassinMainFolders/NPCsSkeletans/Yatch/crewmember2/Animations/CrewmemAnimBP.CrewmemAnimBP_C"))))
    (:`NewEnumerator4`
      (`SkinnedMeshComponent.SetSkinnedAssetAndUpdate` _mesh_4 "/Game/VampireAssassinMainFolders/NPCsSkeletans/Yatch/LifeGuard/Lifeguard_Idle.Lifeguard_Idle" true)
      (`SkeletalMeshComponent.SetAnimInstanceClass` _mesh_4 "/Game/VampireAssassinMainFolders/NPCsSkeletans/Yatch/LifeGuard/Animations/LifeGuardAnimBP.LifeGuardAnimBP_C"))))

(event `self.BouncerDetect.OnComponentBeginOverlap`
  (params (OverlappedComponent :type "PrimitiveComponent Object Reference") (OtherActor :type "Actor Object Reference") (OtherComp :type "PrimitiveComponent Object Reference") (OtherBodyIndex :type Integer) (bFromSweep :type Boolean) (SweepResult :type "HitResult Structure (by ref)"))
  (cast `/Game/AI/Bouncer_AI/BouncerAI` OtherActor)
  (`BlackboardComponent.SetValueAsBool` (`AIBlueprintHelperLibrary.GetBlackboard` null) "OverlapWithBouncer" true))

(event `self.BouncerDetect.OnComponentEndOverlap`
  (params (OverlappedComponent :type "PrimitiveComponent Object Reference") (OtherActor :type "Actor Object Reference") (OtherComp :type "PrimitiveComponent Object Reference") (OtherBodyIndex :type Integer))
  (cast `/Game/AI/Bouncer_AI/BouncerAI` OtherActor)
  (`BlackboardComponent.SetValueAsBool` (`AIBlueprintHelperLibrary.GetBlackboard` null) "OverlapWithBouncer" false))

(fn `UserConstructionScript`
  (`parent.UserConstructionScript`))