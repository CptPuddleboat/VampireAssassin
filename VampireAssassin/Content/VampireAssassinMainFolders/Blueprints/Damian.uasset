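; Damian is the player vampire character, moving relative to a separate Camera actor's yaw.
; An impulse attack that overlaps a DancersBP snaps Damian to its drain point, locking movement and refilling mana on Tick until cancelled.
; A FlipFlop switches between a mana-costing shrink into a rat and a bat Niagara effect.
; It also toggles the pause menu and fires dispatchers for mana, ability and phone changes.
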(event `self.ReceiveBeginPlay`
  (`KismetSystemLibrary.PrintString` "I am in the world" true true (struct :`G` 1.0 :`B` 0.063577 :`A` 1.0))
  (`self.Set Mana`)
  (`self.E_Mana Modified`)
  (bind _returnvalue (`GameplayStatics.GetActorOfClass` "/Game/VampireAssassinMainFolders/Camera/Camera.Camera_C"))
  (set `self.Camera` _returnvalue))

(event `InputAction|RotateCamera`
  (params (Key :type "Key Structure"))
  ;[1 1 1] CameraControl
  (:`Pressed`
    (`/Game/VampireAssassinMainFolders/Camera/Camera.E_CameraRotate` (`self.Camera`) (`self.GetInputAxisValue`))))

(event `InputAction|PauseMenu`
  (params (Key :type "Key Structure"))
  ;[1 1 1] Pause Menu
  (:`Released`
    (`/Engine/EditorBlueprintResources/StandardMacros.FlipFlop`
      (:`A`
        (bind _returnvalue (`|CreateWidget` "/Game/UI_Widgets/LeosUI/UI_MainMenu/PauseWidget.PauseWidget_C"))
        (bind _output_get (set `self.Pause Menu Ref` _returnvalue))
        (`UserWidget.AddToViewport` _output_get 0)
        (`GameplayStatics.SetGamePaused` true)
        (set `PlayerController.bShowMouseCursor` true (`GameplayStatics.GetPlayerController` 0)))
      (:`B`
        (`Widget.RemoveFromParent` (`self.Pause Menu Ref`))
        (set `PlayerController.bShowMouseCursor` false (`GameplayStatics.GetPlayerController` 0))
        (`GameplayStatics.SetGamePaused` false)))))

(event `InputAxis|Up/Down`
  (params (AxisValue :type "Float (single-precision)"))
  ;[1 1 1] Movement
  (if (not (`self.Draining`))
    (`self.AddMovementInput` (`KismetMathLibrary.GetForwardVector` (`KismetMathLibrary.MakeRotator` 0.0 0.0 (.yaw (`self.K2_GetActorRotation` (`self.Camera`))))) AxisValue)))

(event `InputAction|Attack`
  (params (Key :type "Key Structure"))
  ;[1 1 1] Draining Stuff (Copy this)
  (:`Pressed`
    (if (`self.Draining`)
      (set `self.Draining` false)
      (`/Game/VampireAssassinMainFolders/DancingPeople/Male/DancersBP.SetDrain` (`self.DrainingTarget`) false)
      (elif (`self.CanAttack`)
        (set `self.CanAttack` false)
        (set `self.Attacking` true)
        (`CharacterMovementComponent.AddImpulse` (`self.CharacterMovement`) (* (`self.GetActorForwardVector` self) 500000.0) false)
        (`KismetSystemLibrary.K2_SetTimerDelegate` (delegate `ResetAttacking`) 4.0)
        (`KismetSystemLibrary.K2_SetTimerDelegate` (delegate `ResetAttackCooldown`) (`self.AttackCooldown`))))))

(event `ResetAttacking`
  ;[1 1 1] Draining Stuff (Copy this)
  (set `self.Attacking` false)
  (`self.DisableInput` (`GameplayStatics.GetPlayerController` 0)))

(event `InputAxis|Left/Right`
  (params (AxisValue :type "Float (single-precision)"))
  ;[1 1 1] Movement
  (if (not (`self.Draining`))
    (`self.AddMovementInput` (`KismetMathLibrary.GetRightVector` (`KismetMathLibrary.MakeRotator` 0.0 0.0 (.yaw (`self.K2_GetActorRotation` (`self.Camera`))))) AxisValue)))

(event `ResetAttackCooldown`
  ;[1 1 1] Draining Stuff (Copy this)
  (set `self.CanAttack` true)
  (`self.EnableInput` (`GameplayStatics.GetPlayerController` 0)))

(event `self.CapsuleComponent.OnComponentBeginOverlap`
  (params (OverlappedComponent :type "PrimitiveComponent Object Reference") (OtherActor :type "Actor Object Reference") (OtherComp :type "PrimitiveComponent Object Reference") (OtherBodyIndex :type Integer) (bFromSweep :type Boolean) (SweepResult :type "HitResult Structure (by ref)"))
  ;[1 1 1] Draining Stuff (Copy this)
  (bind _asdancers_bp (cast `/Game/VampireAssassinMainFolders/DancingPeople/Male/DancersBP` OtherActor))
  (if (`self.Attacking`)
    (bind _output_get (set `self.DrainingTarget` _asdancers_bp))
    (set `self.Draining` true)
    (`/Game/VampireAssassinMainFolders/DancingPeople/Male/DancersBP.SetDrain` _output_get true)
    (set `MovementComponent.Velocity` (0.0 0.0 0.0) (`self.CharacterMovement`))
    (bind (_returnvalue_location _returnvalue_rotation) (`KismetMathLibrary.BreakTransform` (`SceneComponent.K2_GetComponentToWorld` (`/Game/VampireAssassinMainFolders/DancingPeople/Male/DancersBP.DrainPoint` _output_get))))
    (`self.K2_SetActorLocationAndRotation` _returnvalue_location _returnvalue_rotation)))

(event `InputAction|Activate Ability`
  (params (Key :type "Key Structure"))
  (bind _mesh (`self.Mesh`))
  (bind _rat (`self.Rat`))
  (bind _returnvalue (`self.GetActorScale3D` (`GameplayStatics.GetPlayerCharacter` 0)))
  ;[1 1 1] Ability Press
  (:`Pressed`
    (if (`self.Ability 1 Active`)
      ;;[1 1 1] Ability 1 - Shirnk
      (if (`self.Is Small?`)
        (`self.SetActorScale3D` (+ _returnvalue (0.75 0.75 0.75)))
        (set `self.Is Small?` false)
        (`SceneComponent.SetHiddenInGame` _mesh false false)
        (`SceneComponent.SetHiddenInGame` _rat true false)
        (elif (> (`self.Mana`) 0.0)
          (`SceneComponent.SetHiddenInGame` _mesh true false)
          (`SceneComponent.SetHiddenInGame` _rat false false)
          (`self.SetActorScale3D` (- _returnvalue (0.75 0.75 0.75)))
          (set `self.Is Small?` true)
          (set `self.Mana` (- (`self.Mana`) (`self.Shrink Cost`)))
          (`self.E_Mana Modified`)))
      (elif (`self.Ability 2 Active`)
        (if (`self.Is Small?`)
          _
          (elif (`self.Ability Cooldowned?`)
            (if (> (`self.Mana`) 0.0)
              (set `self.Ability Cooldowned?` false)
              (`NiagaraFunctionLibrary.SpawnSystemAtLocation` "/Game/VampireAssassinMainFolders/Character/Particles/BatsNS.BatsNS" (`SceneComponent.K2_GetComponentLocation` (`Character.Mesh` (`GameplayStatics.GetPlayerCharacter` 0))))
              (`KismetSystemLibrary.Delay` 10.0)
              (set `self.Ability Cooldowned?` false))))))))

(event `InputAction|Change Ability`
  (params (Key :type "Key Structure"))
  ;[1 1 1] Ability Press
  ;;[1 1 1] Change Ability
  (:`Pressed`
    (`/Engine/EditorBlueprintResources/StandardMacros.FlipFlop`
      (:`A`
        (set `self.Ability 1 Active` true)
        (set `self.Ability 2 Active` false)
        (`self.E_Ability 1`))
      (:`B`
        (set `self.Ability 1 Active` false)
        (set `self.Ability 2 Active` true)
        (`self.E_Ability 2`)))))

(event `self.ReceiveTick`
  (params (DeltaSeconds :type "Float (single-precision)"))
  ;[1 1 1] Draining Stuff (Copy this)
  (if (`self.Draining`)
    (bind _output_get (set `self.Mana` (+ (`self.Mana`) (* DeltaSeconds 25.0))))
    (if (> _output_get 100.0)
      (set `self.Mana` 100.0))))

(event `Key|Tab`
  (params (Key :type "Key Structure"))
  ;[1 1 1] Phone
  (:`Pressed`
    (`self.E_Phone Activated`))
  (:`Released`
    (`self.E_Phone Deactivated`)))

(fn `Set HUD`
  (bind _returnvalue (`|CreateWidget` "/Game/VampireAssassinMainFolders/Character/UI/HUD.HUD_C" (`GameplayStatics.GetPlayerController` 0)))
  (`UserWidget.AddToViewport` _returnvalue 0))

(fn `Set Mana`
  (set `self.Max Mana` (`self.Max Mana`))
  (set `self.Mana` (`self.Mana`)))

(fn `UserConstructionScript`)