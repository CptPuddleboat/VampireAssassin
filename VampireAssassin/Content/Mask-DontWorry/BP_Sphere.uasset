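; BP_Sphere is a sphere mask controller that publishes its position and size to the PC_Data material parameter collection.
; The construction script and MaskLocation event write the Sphere's world location and X scale to "Position 1" and "Radius".
; BeginPlay caches an ActorLocation actor, whose root location GoAway writes to "Position 1" to move the mask away, leaving the radius unchanged.
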(event `self.ReceiveBeginPlay`
  (bind _returnvalue (`GameplayStatics.GetActorOfClass` "/Game/Mask-DontWorry/ActorLocation.ActorLocation_C"))
  (set `self.HideLocationRef` _returnvalue))

(event `GoAway`
  (`KismetMaterialLibrary.SetVectorParameterValue` "/Game/Mask-DontWorry/PC_Data.PC_Data" "Position 1" (`KismetMathLibrary.Conv_VectorToLinearColor` (`SceneComponent.K2_GetComponentLocation` (`/Game/Mask-DontWorry/ActorLocation.DefaultSceneRoot` (`self.HideLocationRef`))))))

(event `MaskLocation`
  (bind _sphere (`self.Sphere`))
  (bind _returnvalue_x (`KismetMathLibrary.BreakVector` (`SceneComponent.K2_GetComponentScale` _sphere)))
  (`KismetMaterialLibrary.SetVectorParameterValue` "/Game/Mask-DontWorry/PC_Data.PC_Data" "Position 1" (`KismetMathLibrary.Conv_VectorToLinearColor` (`SceneComponent.K2_GetComponentLocation` _sphere)))
  (`KismetMaterialLibrary.SetScalarParameterValue` "/Game/Mask-DontWorry/PC_Data.PC_Data" "Radius" _returnvalue_x))

(fn `UserConstructionScript`
  (bind _sphere (`self.Sphere`))
  (bind _returnvalue_x (`KismetMathLibrary.BreakVector` (`SceneComponent.K2_GetComponentScale` _sphere)))
  (`KismetMaterialLibrary.SetVectorParameterValue` "/Game/Mask-DontWorry/PC_Data.PC_Data" "Position 1" (`KismetMathLibrary.Conv_VectorToLinearColor` (`SceneComponent.K2_GetComponentLocation` _sphere)))
  (`KismetMaterialLibrary.SetScalarParameterValue` "/Game/Mask-DontWorry/PC_Data.PC_Data" "Radius" _returnvalue_x))