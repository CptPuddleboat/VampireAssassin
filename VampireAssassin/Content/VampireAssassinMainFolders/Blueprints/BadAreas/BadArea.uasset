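; BadArea is a zone actor that flags the Damian actor as being in a bad area.
; Its StaticMesh begin overlap sets InBadArea on Damian, and end overlap clears it only when Damian's Mesh is the exiting component.
; Tick prints display names from the NewVar0 array as debug output, and disconnected DoOnce logic for the same flag never runs.
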(event `self.StaticMesh.OnComponentBeginOverlap`
  (params (OverlappedComponent :type "PrimitiveComponent Object Reference") (OtherActor :type "Actor Object Reference") (OtherComp :type "PrimitiveComponent Object Reference") (OtherBodyIndex :type Integer) (bFromSweep :type Boolean) (SweepResult :type "HitResult Structure (by ref)"))
  (bind _asdamian (cast `/Game/VampireAssassinMainFolders/Character/PlayerCharacter/Damian` OtherActor))
  (set `/Game/VampireAssassinMainFolders/Character/PlayerCharacter/Damian.In Bad Area` true _asdamian))

(event `self.ReceiveTick`
  (params (DeltaSeconds :type "Float (single-precision)"))
  (for _array_element (`self.NewVar_0`)
    (`KismetSystemLibrary.PrintString` (`KismetSystemLibrary.GetDisplayName` _array_element))))

(event `self.StaticMesh.OnComponentEndOverlap`
  (params (OverlappedComponent :type "PrimitiveComponent Object Reference") (OtherActor :type "Actor Object Reference") (OtherComp :type "PrimitiveComponent Object Reference") (OtherBodyIndex :type Integer))
  (bind _asdamian (cast `/Game/VampireAssassinMainFolders/Character/PlayerCharacter/Damian` OtherActor))
  (if (== (`Character.Mesh` _asdamian) OtherComp)
    (set `/Game/VampireAssassinMainFolders/Character/PlayerCharacter/Damian.In Bad Area` false _asdamian)))

(fn `UserConstructionScript`)